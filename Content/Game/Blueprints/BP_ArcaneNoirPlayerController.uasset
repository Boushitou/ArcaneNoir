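; Player controller for Arcane Noir that toggles the inventory and stats menu widgets from Enhanced Input actions.
; On BeginPlay it caches the ArcaneNoir HUD, which holds both widgets, and sets game-only input with permanent mouse capture.
; Each toggle adds or removes its widget from the viewport, switching to game-and-UI input focused on it when opened and restoring game-only capture when closed.
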(event Input|EnhancedActionEvents|EnhancedInputActionIA_OpenInventory
  (params (ActionValue :type Boolean) (ElapsedSeconds :type Float%20%28double-precision%29) (TriggeredSeconds :type Float%20%28double-precision%29) (InputAction :type Input%20Action%20Object%20Reference :default "/Game/Game/Input/Actions/Menus/IA_OpenInventory.IA_OpenInventory"))
  (:Started
    (CallFunction|OpenInventory)))

(event Input|EnhancedActionEvents|EnhancedInputActionIA_OpenStatsMenu
  (params (ActionValue :type Boolean) (ElapsedSeconds :type Float%20%28double-precision%29) (TriggeredSeconds :type Float%20%28double-precision%29) (InputAction :type Input%20Action%20Object%20Reference :default "/Game/Game/Input/Actions/Menus/IA_OpenStatsMenu.IA_OpenStatsMenu"))
  (:Started
    (CallFunction|OpenStatsMenu)))

(event Input|EnhancedActionEvents|EnhancedInputActionIA_SetDestination_Click
  (params (ActionValue :type Boolean) (ElapsedSeconds :type Float%20%28double-precision%29) (TriggeredSeconds :type Float%20%28double-precision%29) (InputAction :type Input%20Action%20Object%20Reference :default "/Game/Game/Input/Actions/Player/IA_SetDestination_Click.IA_SetDestination_Click")))

(event EventBeginPlay
  (bind _asarcane_noir_hud (Utilities|Casting|CastToArcaneNoir_HUD (HUD|GetHUD)))
  (Variables|Default|SetArcane%20Noir%20HUD _asarcane_noir_hud)
  (Input|SetInputModeGameOnly self true)
  (Class|GameplayStatics|SetViewportMouseCaptureMode "CapturePermanently_IncludingInitialMouseDown"))

(event EventTick
  (params (DeltaSeconds :type Float%20%28single-precision%29)))

(fn ConstructionScript)

(fn OpenInventory
  (bind _self self)
  (bind _arcane_noir_hud (Variables|Default|GetArcane%20Noir%20HUD))
  (bind _inventory (Variables|/Game/Game/UI/ArcaneNoir_HUD.ArcaneNoir_HUD_C|GetInventory _arcane_noir_hud))
  (if (UserInterface|Viewport|IsinViewport _inventory)
    (Widget|RemovefromParent _inventory)
    (Input|SetInputModeGameOnly _self true)
    (Class|GameplayStatics|SetViewportMouseCaptureMode "CapturePermanently_IncludingInitialMouseDown")
    (else
      (UserInterface|Viewport|AddtoViewport _inventory 0)
      (Input|SetInputModeGameandUI _self (Variables|/Game/Game/UI/ArcaneNoir_HUD.ArcaneNoir_HUD_C|GetInventory (Variables|Default|GetArcane%20Noir%20HUD)) "DoNotLock" false true))))

(fn OpenStatsMenu
  (bind _arcane_noir_hud (Variables|Default|GetArcane%20Noir%20HUD))
  (bind _statsmenu (Variables|/Game/Game/UI/ArcaneNoir_HUD.ArcaneNoir_HUD_C|GetStatsMenu _arcane_noir_hud))
  (if (UserInterface|Viewport|IsinViewport (Variables|/Game/Game/UI/ArcaneNoir_HUD.ArcaneNoir_HUD_C|GetStatsMenu (Variables|Default|GetArcane%20Noir%20HUD)))
    (Widget|RemovefromParent _statsmenu)
    (Input|SetInputModeGameOnly 0 true)
    (Class|GameplayStatics|SetViewportMouseCaptureMode "CapturePermanently_IncludingInitialMouseDown")
    (else
      (UserInterface|Viewport|AddtoViewport _statsmenu 0)
      (Input|SetInputModeGameandUI self _statsmenu "DoNotLock" false false))))